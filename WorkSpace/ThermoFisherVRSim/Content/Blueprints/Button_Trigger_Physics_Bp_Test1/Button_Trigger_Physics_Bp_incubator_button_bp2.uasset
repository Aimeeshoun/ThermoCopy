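; A physics trigger button, apparently a test for an incubator button, whose mesh sinks while actors overlap its box and rises when the box is empty.
; Each Tick polls the box overlaps and steps the mesh's relative Z with a near-instant MoveComponentTo, clamped between zero and an offset variable.
; The construction script uses that offset for the arrow length and the mesh's raised starting height.
; The graph only moves the mesh and signals nothing else.
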(event EventTick
  (params (DeltaSeconds :type Float%20%28single-precision%29))
  (bind _staticmesh (Variables|Default|GetStaticMesh))
  (bind _staticmesh_2 (Variables|Default|GetStaticMesh))
  ;[1 1 1] Comment
  (if (> (Utilities|Array|Length (Collision|GetOverlappingActors (Variables|Default|GetBox) 0 :!class /Script/Engine.PrimitiveComponent)) 0)
    (Components|MoveComponentTo _staticmesh_2 (Math|Vector|MakeVector 0.0 0.0 (Math|Float|Clamp(Float) (- (.z (Variables|/Script/Engine.SceneComponent|GetRelativeLocation _staticmesh_2)) 3.0) 0.0 (Variables|Default|GetButton_Offset_Test1))) (Math|Rotator|MakeRotator 0.0 0.0 0.0) true true 0.0001 false)
    (else
      (Components|MoveComponentTo _staticmesh (Math|Vector|MakeVector 0.0 0.0 (Math|Float|Clamp(Float) (+ (.z (Variables|/Script/Engine.SceneComponent|GetRelativeLocation _staticmesh)) 3.0) 0.0 (Variables|Default|GetButton_Offset_Test1))) "0, 0, 0" true true 0.0001 false))))

(fn ConstructionScript
  (bind _button_offset_test1 (Variables|Default|GetButton_Offset_Test1))
  ;[1 1 1] Comment
  (Variables|/Script/Engine.ArrowComponent|SetArrowLength (Variables|Default|GetArrow_test1) _button_offset_test1)
  (Transformation|SetRelativeLocation (Variables|Default|GetStaticMesh) (Math|Vector|MakeVector 0.0 0.0 _button_offset_test1) false false))