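; Test Blueprint for a physical button that responds to actors overlapping its trigger box.
; Each Tick checks the box and calls MoveComponentTo with the button mesh's Z location clamped between zero and the button offset.
; When overlapped, that value drives the mesh's target yaw; otherwise it becomes a target Z location with no component assigned.
; The construction script sizes an arrow to the offset, leaving a mesh-positioning call unexecuted.
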(event EventTick
  (params (DeltaSeconds :type Float%20%28single-precision%29))
  (bind _button_button_mesh_test1 (Variables|Default|GetButton_Button_Mesh_test1))
  ;[1 1 1] Comment
  (if (> (Utilities|Array|Length (Collision|GetOverlappingActors (Variables|Default|Getbutton_Trigger_box_test1) 0 :!class /Script/Engine.PrimitiveComponent)) 0)
    (Components|MoveComponentTo _button_button_mesh_test1 "0, 0, 0" (Math|Rotator|MakeRotator 0.0 0.0 (Math|Float|Clamp(Float) (- (.z (Variables|/Script/Engine.SceneComponent|GetRelativeLocation _button_button_mesh_test1)) 0.0) 0.0 (Variables|Default|GetButton_Offset_Test1))) false false 0.0001 false)
    (else
      (Components|MoveComponentTo 0 (Math|Vector|MakeVector 0.0 0.0 (Math|Float|Clamp(Float) (+ (.z (Variables|/Script/Engine.SceneComponent|GetRelativeLocation (Variables|Default|GetButton_Button_Mesh_test1))) 0.0) 0.0 (Variables|Default|GetButton_Offset_Test1))) "0, 0, 0" false false 0.2 false))))

(fn ConstructionScript
  ;[1 1 1] Comment
  (Variables|/Script/Engine.ArrowComponent|SetArrowLength (Variables|Default|GetArrow_test1) (Variables|Default|GetButton_Offset_Test1)))