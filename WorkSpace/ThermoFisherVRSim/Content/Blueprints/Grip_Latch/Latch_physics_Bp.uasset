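; Latch actor Blueprint, apparently a VR grip-latch prototype, that moves its Lever component when something overlaps its Box trigger.
; The overlap event prints a debug string and eases the Lever to a rotation derived from its current relative rotation, keeping its location.
; It queries left motion controller data without using the result.
; An unconnected overlap check with an instant pitch rotation remains in the graph but never runs.
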(event OnComponentBeginOverlap(Box)
  (params (OverlappedComponent :type Primitive%20Component%20Object%20Reference) (OtherActor :type Actor%20Object%20Reference) (OtherComp :type Primitive%20Component%20Object%20Reference) (OtherBodyIndex :type Integer) (bFromSweep :type Boolean) (SweepResult :type Hit%20Result%20Structure%20%28by%20ref%29))
  (bind _lever (Variables|Default|Getlever))
  (bind _returnvalue (Transformation|GetRelativeTransform _lever))
  (Class|HeadMountedDisplayFunctionLibrary|GetMotionControllerData OverlappedComponent "Left")
  (Development|PrintString "lever")
  (Components|MoveComponentTo _lever (.location _returnvalue) (Math|Conversions|RotationFromXVector (- (.rotation _returnvalue) "0,0.000000,90.000000")) false true 0.8 false))

(event EventBeginPlay)

(event Collision|EventActorBeginOverlap
  (params (OtherActor :type Actor%20Object%20Reference)))

(event EventTick
  (params (DeltaSeconds :type Float%20%28single-precision%29)))

(event Input|ActionEvents|InputActionLatch_interaction
  (params (Key :type Key%20Structure :default "None")))

(fn ConstructionScript)