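; Lever actor whose stick follows a motion controller, swinging on a single pitch axis.
; Each Tick, while a MotionController reference is valid, it converts the controller's position into the stick's rotated local space and takes the look-at pitch.
; That pitch is added to the stick's current relative pitch and clamped to a quarter turn, with roll and yaw held at zero.
; The graph never assigns the controller reference itself.
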(event EventTick
  (params (DeltaSeconds :type Float%20%28single-precision%29))
  (bind _lever_stick (Variables|Default|Getlever_stick))
  (bind _lever_stick_2 (Variables|Default|Getlever_stick))
  (bind _returnvalue (Transformation|GetWorldTransform _lever_stick))
  (bind _motion_controller (Variables|Default|GetMotion_Controller)
    (:then
      (Transformation|SetRelativeRotation _lever_stick_2 (Math|Rotator|MakeRotator 0.0 (Math|Float|Clamp(Float) (+ (.pitch (Variables|/Script/Engine.SceneComponent|GetRelativeRotation _lever_stick_2)) (.pitch (Math|Rotator|FindLookatRotation (Math|Vector|MakeVector 0.0 0.0 0.0) (.location (Math|Transform|MakeRelativeTransform (Transformation|GetWorldTransform _motion_controller) (Math|Transform|MakeTransform (.location _returnvalue) (Math|Rotator|CombineRotators (.rotation _returnvalue) "90.000000, 0, 0") (.scale _returnvalue))))))) 0.0 9e+01) 0.0) false false))
    (:else)))

(fn ConstructionScript)