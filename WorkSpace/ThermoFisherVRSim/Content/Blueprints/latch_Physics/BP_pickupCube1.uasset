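; Latch or lever physics prototype that moves its Level component according to whether anything overlaps its Box.
; Each Tick uses MoveComponentTo to step Level's pitch down within a clamp while overlapped, otherwise deriving height and pitch targets from its relative Y location.
; Overlap events set and print LeverGrabbed, which nothing reads; Pickup and Drop store or clear a motion controller.
; Controller-following look-at rotation logic is present but disconnected.
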(event OnComponentHit(Box)
  (params (HitComponent :type Primitive%20Component%20Object%20Reference) (OtherActor :type Actor%20Object%20Reference) (OtherComp :type Primitive%20Component%20Object%20Reference) (NormalImpulse :type Vector :default "0, 0, 0") (Hit :type Hit%20Result%20Structure%20%28by%20ref%29)))

(event OnComponentBeginOverlap(Box)
  (params (OverlappedComponent :type Primitive%20Component%20Object%20Reference) (OtherActor :type Actor%20Object%20Reference) (OtherComp :type Primitive%20Component%20Object%20Reference) (OtherBodyIndex :type Integer) (bFromSweep :type Boolean) (SweepResult :type Hit%20Result%20Structure%20%28by%20ref%29))
  ;[1 1 1] Comment
  (Variables|Default|SetLever_Grabbed true)
  (Development|PrintString "overlapped"))

(event OnComponentEndOverlap(Box)
  (params (OverlappedComponent :type Primitive%20Component%20Object%20Reference) (OtherActor :type Actor%20Object%20Reference) (OtherComp :type Primitive%20Component%20Object%20Reference) (OtherBodyIndex :type Integer))
  ;[1 1 1] Comment
  (Variables|Default|SetLever_Grabbed false)
  (Development|PrintString "not overlapped"))

(event EventBeginPlay)

(event Collision|EventActorBeginOverlap
  (params (OtherActor :type Actor%20Object%20Reference)))

(event EventPickup
  (params (right_controller :type Motion%20Controller%20Component%20Object%20Reference) (left_controller :type Motion%20Controller%20Component%20Object%20Reference))
  ;[1 1 1] Comment
  (Variables|Default|Setleft_motion_controller left_controller))

(event EventDrop
  (params (left_controller :type Motion%20Controller%20Component%20Object%20Reference) (right_controller :type Motion%20Controller%20Component%20Object%20Reference))
  ;[1 1 1] Comment
  (if (== (Variables|Default|Getleft_motion_controller) left_controller)
    (Variables|Default|Setleft_motion_controller 0)))

(event EventTick
  (params (DeltaSeconds :type Float%20%28single-precision%29))
  (bind _level (Variables|Default|Getlevel))
  (bind _level_2 (Variables|Default|Getlevel))
  (bind _relativelocation (Variables|/Script/Engine.SceneComponent|GetRelativeLocation _level))
  (if (> (Utilities|Array|Length (Collision|GetOverlappingActors (Variables|Default|GetBox) 0 :!class /Script/Engine.PrimitiveComponent)) 0)
    (Components|MoveComponentTo _level_2 (Math|Vector|MakeVector 0.0 0.0 0.0) (Math|Rotator|MakeRotator 0.0 (Math|Float|Clamp(Float) (- (.pitch (Variables|/Script/Engine.SceneComponent|GetRelativeRotation _level_2)) 3.0) 0.0 9e+01) 0.0) true true 0.0001 false)
    (else
      (Components|MoveComponentTo _level (Math|Vector|MakeVector 0.0 0.0 (Math|Float|Clamp(Float) (+ (.y _relativelocation) 3.0) 0.0 9e+01)) (Math|Rotator|MakeRotator 0.0 (.y _relativelocation) 0.0) true true 0.0001 false))))

(fn ConstructionScript)