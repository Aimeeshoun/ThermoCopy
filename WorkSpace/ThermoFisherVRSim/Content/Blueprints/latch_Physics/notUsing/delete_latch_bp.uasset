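; A latch Blueprint whose body swings in yaw while actors overlap its trigger box and swings back when the box is empty.
; Tick steps the yaw down or up by a fixed amount, clamped between zero and ButtonOffsetTest1, through near-instant MoveComponentTo calls.
; The construction script starts the body at that offset and reuses the value as the length of an arrow component.
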(event EventTick
  (params (DeltaSeconds :type Float%20%28single-precision%29))
  (bind _latch_body (Variables|Default|Getlatch_body))
  (bind _latch_body_2 (Variables|Default|Getlatch_body))
  ;[1 1 1] Comment
  (if (> (Utilities|Array|Length (Collision|GetOverlappingActors (Variables|Default|GetBox_Trigger) 0 :!class /Script/Engine.PrimitiveComponent)) 0)
    (Components|MoveComponentTo _latch_body_2 (Math|Vector|MakeVector 0.0 0.0 0.0) (Math|Rotator|MakeRotator 0.0 0.0 (Math|Float|Clamp(Float) (- (.yaw (Variables|/Script/Engine.SceneComponent|GetRelativeRotation _latch_body_2)) 3.0) 0.0 (Variables|Default|GetButton_Offset_Test1))) true true 0.0001 false)
    (else
      (Components|MoveComponentTo _latch_body (Math|Vector|MakeVector 0.0 0.0 0.0) (Math|Rotator|MakeRotator 0.0 0.0 (Math|Float|Clamp(Float) (+ (.yaw (Variables|/Script/Engine.SceneComponent|GetRelativeRotation _latch_body)) 3.0) 0.0 (Variables|Default|GetButton_Offset_Test1))) true true 0.0001 false))))

(fn ConstructionScript
  (bind _button_offset_test1 (Variables|Default|GetButton_Offset_Test1))
  ;[1 1 1] Comment
  (Variables|/Script/Engine.ArrowComponent|SetArrowLength (Variables|Default|GetArrow_test1) _button_offset_test1)
  (Transformation|SetRelativeRotation (Variables|Default|Getlatch_body) (Math|Rotator|MakeRotator 0.0 0.0 _button_offset_test1) false false))