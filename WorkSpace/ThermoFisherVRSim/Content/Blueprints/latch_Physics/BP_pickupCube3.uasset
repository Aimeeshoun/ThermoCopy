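; VR lever prototype that rotates its Level component when GrabLeft is pressed while the Box trigger is overlapped.
; Box overlap events toggle LeverGrabbed, and each press adds the look-at pitch toward Arrow1, in Level's yaw-offset space, to the current pitch, clamped to a quarter turn.
; Pickup and Drop store and clear the left controller, but the rotation never uses it.
; Debug prints report overlaps and the computed angle.
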(event OnComponentBeginOverlap(Box)
  (params (OverlappedComponent :type Primitive%20Component%20Object%20Reference) (OtherActor :type Actor%20Object%20Reference) (OtherComp :type Primitive%20Component%20Object%20Reference) (OtherBodyIndex :type Integer) (bFromSweep :type Boolean) (SweepResult :type Hit%20Result%20Structure%20%28by%20ref%29))
  ;[1 1 1] Comment
  (Variables|Default|SetLever_Grabbed true)
  (Development|PrintString "overlapped"))

(event OnComponentEndOverlap(Box)
  (params (OverlappedComponent :type Primitive%20Component%20Object%20Reference) (OtherActor :type Actor%20Object%20Reference) (OtherComp :type Primitive%20Component%20Object%20Reference) (OtherBodyIndex :type Integer))
  ;[1 1 1] Comment
  (Variables|Default|SetLever_Grabbed false)
  (Development|PrintString "not overlapped"))

(event EventBeginPlay)

(event Collision|EventActorBeginOverlap
  (params (OtherActor :type Actor%20Object%20Reference)))

(event EventPickup
  (params (right_controller :type Motion%20Controller%20Component%20Object%20Reference) (left_controller :type Motion%20Controller%20Component%20Object%20Reference))
  ;[1 1 1] Comment
  (Variables|Default|Setleft_motion_controller left_controller))

(event EventDrop
  (params (left_controller :type Motion%20Controller%20Component%20Object%20Reference) (right_controller :type Motion%20Controller%20Component%20Object%20Reference))
  ;[1 1 1] Comment
  (if (== (Variables|Default|Getleft_motion_controller) left_controller)
    (Variables|Default|Setleft_motion_controller 0)))

(event Input|ActionEvents|InputActionGrabLeft
  (params (Key :type Key%20Structure :default "None"))
  (bind _returnvalue (Math|Vector|MakeVector 0.0 0.0 0.0))
  (bind _level (Variables|Default|Getlevel))
  (bind _level_2 (Variables|Default|Getlevel))
  (bind _arrow1 (Variables|Default|GetArrow1))
  (bind _returnvalue_2 (Transformation|GetWorldTransform _arrow1))
  (bind _returnvalue_3 (Transformation|GetWorldTransform _level_2))
  (bind _relativerotation (Variables|/Script/Engine.SceneComponent|GetRelativeRotation _level))
  (bind _returnvalue_4 (Math|Rotator|CombineRotators (.rotation _returnvalue_3) "90.000000, 0, 0"))
  (bind _returnvalue_5 (Math|Transform|MakeRelativeTransform _returnvalue_2 (Math|Transform|MakeTransform (.location _returnvalue_3) _returnvalue_4 (.scale _returnvalue_3))))
  (bind _returnvalue_6 (Math|Rotator|FindLookatRotation _returnvalue (.location _returnvalue_5)))
  (bind _returnvalue_7 (+ (.pitch _relativerotation) (.pitch _returnvalue_6)))
  (bind _returnvalue_8 (Math|Float|Clamp(Float) _returnvalue_7 0.0 9e+01))
  ;[1 1 1] Comment
  (:Pressed
    (if (Variables|Default|GetLever_Grabbed)
      (if (> (Utilities|Array|Length (Collision|GetOverlappingActors (Variables|Default|GetBox) 0 :!class /Script/Engine.PrimitiveComponent)) 0)
        (Transformation|SetWorldRotation (Variables|Default|Getlevel) (Math|Rotator|MakeRotator 0.0 _returnvalue_8 0.0) false false)
        (Development|PrintString (Utilities|String|ToString(Float) _returnvalue_8))))))

(fn ConstructionScript)