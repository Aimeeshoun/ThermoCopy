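; Prototype VR latch or lever that a motion controller grabs to rotate its Level component.
; Pickup stores the left controller and Drop clears it when the passed controllers match the stored references.
; While that controller is valid, Tick adds the Arrow-to-Cube roll difference to Level's pitch, clamped to a quarter turn.
; Box overlaps and Pickup set LeverGrabbed, which nothing reads; right-controller assignment is unwired, and debug prints remain.
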(event OnComponentBeginOverlap(Box)
  (params (OverlappedComponent :type Primitive%20Component%20Object%20Reference) (OtherActor :type Actor%20Object%20Reference) (OtherComp :type Primitive%20Component%20Object%20Reference) (OtherBodyIndex :type Integer) (bFromSweep :type Boolean) (SweepResult :type Hit%20Result%20Structure%20%28by%20ref%29))
  ;[1 1 1] Comment
  (Variables|Default|SetLever_Grabbed true)
  (Development|PrintString "overlapped"))

(event OnComponentEndOverlap(Box)
  (params (OverlappedComponent :type Primitive%20Component%20Object%20Reference) (OtherActor :type Actor%20Object%20Reference) (OtherComp :type Primitive%20Component%20Object%20Reference) (OtherBodyIndex :type Integer))
  ;[1 1 1] Comment
  (Variables|Default|SetLever_Grabbed false)
  (Development|PrintString "not overlapped"))

(event EventBeginPlay)

(event Collision|EventActorBeginOverlap
  (params (OtherActor :type Actor%20Object%20Reference)))

(event EventPickup
  (params (right_controller :type Motion%20Controller%20Component%20Object%20Reference) (left_controller :type Motion%20Controller%20Component%20Object%20Reference))
  ;[1 1 1] Comment
  (Variables|Default|SetLever_Grabbed true)
  (Variables|Default|Setleft_motion_controller left_controller))

(event EventDrop
  (params (left_controller :type Motion%20Controller%20Component%20Object%20Reference) (right_controller :type Motion%20Controller%20Component%20Object%20Reference))
  ;[1 1 1] Comment
  (if (and (== (Variables|Default|Getleft_motion_controller) left_controller) (== (Variables|Default|Getright_motion_controller) right_controller))
    (Variables|Default|Setleft_motion_controller 0)))

(event EventTick
  (params (DeltaSeconds :type Float%20%28single-precision%29))
  (bind _arrow (Variables|Default|GetArrow))
  (bind _level (Variables|Default|Getlevel))
  (bind _cube (Variables|Default|GetCube))
  (bind _returnvalue (Transformation|GetWorldRotation _cube))
  (bind _returnvalue_2 (Transformation|GetWorldRotation _level))
  (bind _returnvalue_3 (Transformation|GetWorldRotation _arrow))
  (bind _returnvalue_4 (- (.roll _returnvalue_3) (.roll _returnvalue)))
  (bind _returnvalue_5 (+ (.pitch _returnvalue_2) _returnvalue_4))
  (bind _returnvalue_6 (Math|Float|Clamp(Float) _returnvalue_5 0.0 9e+01))
  ;[1 1 1] Comment
  (Variables|Default|Getleft_motion_controller
    (:then
      (Transformation|SetWorldRotation _level (Math|Rotator|MakeRotator (.roll _returnvalue_2) _returnvalue_6 (.yaw _returnvalue_2)) false false)
      (Development|PrintString (Utilities|String|ToString(Float) _returnvalue_6)))
    (:else)))

(fn ConstructionScript)