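; InteractiveDoor is an interactable door that slides open and closed, toggling each time its Interact event fires.
; Interact flips InteractState and plays or reverses a timeline, whose DoorInterpolation track lerps the Door component's relative location between StartLocation and EndLocation.
; GetInteractState returns a variable named State rather than the InteractState flag that Interact toggles.
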(event EventBeginPlay)

(event Collision|EventActorBeginOverlap
  (params (OtherActor :type Actor%20Object%20Reference)))

(event EventTick
  (params (DeltaSeconds :type Float%20%28single-precision%29)))

(event EventInteract
  (if (Variables|Default|GetInteract_state)
    (Variables|Default|SetInteract_state false)
    (bind _door_interpolation (Timeline|Timeline_0 Reverse)
      (:Update
        (Transformation|SetRelativeLocation (Variables|Default|Getdoor) (Math|Vector|Lerp(Vector) (Variables|Default|GetStart_location) (Variables|Default|Getend_location) _door_interpolation) false false)))
    (else
      (Variables|Default|SetInteract_state true)
      (Timeline|Timeline_0 Play))))

(fn ConstructionScript)

(fn GetInteractState
  (return (Variables|Default|GetState)))